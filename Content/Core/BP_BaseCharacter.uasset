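; Base player character with step-based movement: forward/back input moves it a set distance, and sideways input turns it by a set yaw step.
; Tick interpolates toward the target location with a swept move, resetting the target if the move fails; new steps wait until the target is reached.
; Helper functions squash and restore mesh Z scale, return it to its start position, or raise it to a fixed height above that start.
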(event Input|EnhancedActionEvents|EnhancedInputActionIA_Player
  (params (ActionValue :type Vector%202D%20Structure) (ElapsedSeconds :type Float%20%28double-precision%29) (TriggeredSeconds :type Float%20%28double-precision%29) (InputAction :type Input%20Action%20Object%20Reference :default "/Game/Core/Input/IA_Player.IA_Player"))
  (bind (_x _y) (Math|Vector2D|BreakVector2D ActionValue))
  (:Triggered
    (if (Utilities|Operators|EqualEqual (Variables|Default|GetTargetLocation) (Transformation|GetActorLocation) 0.1)
      (Variables|Default|SetTargetLocation (+ (* (Transformation|GetActorForwardVector) (* _y (Variables|Default|GetLocationDelta))) (Transformation|GetActorLocation)))))
  (:Started
    (Class|Actor|AddActorWorldRotation (Math|Rotator|MakeRotator 0.0 0.0 (* _x (Variables|Default|GetRotationDelta))))))

(event EventBeginPlay
  (Input|AddMappingContext (PlayerController|LocalPlayerSubsystems|GetEnhancedInputLocalPlayerSubsystem (Game|GetPlayerController 0)) "/Game/Core/Input/IMC_Player.IMC_Player" 0 "(bIgnoreAllPressedKeysUntilRelease=True,bForceImmediately=False,bNotifyUserSettings=False)")
  (Variables|Default|SetTargetLocation (Transformation|GetActorLocation))
  (Variables|Default|SetOriginal_Scale (Variables|/Script/Engine.SceneComponent|GetRelativeScale3D (Variables|Default|GetStaticMesh)))
  (Variables|Default|SetPlayerStartLocation (Transformation|GetActorLocation)))

(event Collision|EventActorBeginOverlap
  (params (OtherActor :type Actor%20Object%20Reference)))

(event EventTick
  (params (DeltaSeconds :type Float%20%28single-precision%29))
  (bind _returnvalue (Transformation|SetActorLocation (Math|Interpolation|VInterpTo (Transformation|GetActorLocation) (Variables|Default|GetTargetLocation) DeltaSeconds (Variables|Default|GetMovementInterpolationSpeed)) true false))
  (if (not _returnvalue)
    (Variables|Default|SetTargetLocation (Transformation|GetActorLocation))))

(fn ConstructionScript)

(fn ScaleZ
  (bind _staticmesh (Variables|Default|GetStaticMesh))
  (bind _relativescale3d (Variables|/Script/Engine.SceneComponent|GetRelativeScale3D _staticmesh))
  (Transformation|SetRelativeScale3D _staticmesh (Math|Vector|MakeVector (.x _relativescale3d) (.y _relativescale3d) (* (.z _relativescale3d) 0.2))))

(fn ReturnScale
  (Transformation|SetRelativeScale3D (Variables|Default|GetStaticMesh) (Variables|Default|GetOriginal_Scale)))

(fn ReturntoStart
  (Transformation|SetActorLocation (Variables|Default|GetPlayerStartLocation) false false)
  ;[1 1 1] ne nravitsa
  (Variables|Default|SetTargetLocation (Variables|Default|GetPlayerStartLocation)))

(fn Levitation
  (bind _returnvalue (Transformation|GetActorLocation))
  (bind _playerstartlocation (Variables|Default|GetPlayerStartLocation))
  (bind _returnvalue_2 (+ (.z _playerstartlocation) 2.5e+02))
  (Transformation|SetActorLocation (Math|Vector|MakeVector (.x _returnvalue) (.y _returnvalue) _returnvalue_2) false false)
  (Variables|Default|SetTargetLocation (Math|Vector|MakeVector (.x _returnvalue) (.y _returnvalue) _returnvalue_2)))