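; BP_Crusher is a crusher hazard that moves vertically and squashes any BP_BaseCharacter its mesh overlaps.
; BeginPlay stores the origin and starts a timeline, rate-scaled by Time, whose ZAxis track times Offset sets the height.
; On overlap it calls the character's ScaleZ, then ReturnToStart and ReturnScale after short delays.
; An earlier VInterpTo movement approach remains as unconnected nodes.
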(event OnComponentBeginOverlap(StaticMesh)
  (params (OverlappedComponent :type Primitive%20Component%20Object%20Reference) (OtherActor :type Actor%20Object%20Reference) (OtherComp :type Primitive%20Component%20Object%20Reference) (OtherBodyIndex :type Integer) (bFromSweep :type Boolean) (SweepResult :type Hit%20Result%20Structure%20%28by%20ref%29))
  (bind _asbp_base_character (Utilities|Casting|CastToBP_BaseCharacter OtherActor))
  (Default|ScaleZ _asbp_base_character)
  (Utilities|FlowControl|Delay 0.2)
  (Default|ReturntoStart _asbp_base_character)
  (Utilities|FlowControl|Delay 0.3)
  (Default|ReturnScale _asbp_base_character))

(event EventBeginPlay
  (Variables|Default|SetOriginPosition (Transformation|GetActorLocation))
  (Components|Timeline|SetPlayRate (Variables|Default|GetTimeline) (/ 1.0 (Variables|Default|GetTime)))
  (Components|Timeline|PlayfromStart (Variables|Default|GetTimeline)))

(fn ConstructionScript)